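; BP_IPGPlayerController is the player controller that bootstraps the game's UI when play begins.
; On BeginPlay it creates the primary layout widget, adds it to the viewport and registers it with the IPGUISubsystem.
; It then pushes a soft-referenced guild screen, looked up by gameplay tag, onto the front-end widget stack as the opening screen.
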(event `self.ReceiveBeginPlay`
  (bind _returnvalue (`|CreateWidget` "/Game/UI/WBP_PrimaryLayout.WBP_PrimaryLayout_C" self))
  (bind _output_get (set `self.PrimaryLayoutWidget` _returnvalue))
  (`/Engine/EditorBlueprintResources/StandardMacros.IsValid` _output_get
    (:`Is Valid`
      (`UserWidget.AddToViewport` (`self.PrimaryLayoutWidget`) 0)
      (`IPGUISubsystem.RegisterCreatedPrimaryLayoutWidget` (subsystem `IPGUISubsystem`) (`self.PrimaryLayoutWidget`))
      (`PushSoftWidgetAsyncAction.PushSoftWidget` self (`IPGUIFunctionLibrary.GetIPGSoftWidgetClassByTag` (struct :`TagName` "UI.Widget.GuildScreen")) (struct :`TagName` "UI.WidgetStack.FrontEnd")))))

(fn `UserConstructionScript`)