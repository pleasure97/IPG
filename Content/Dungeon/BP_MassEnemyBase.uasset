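; Base Blueprint for dungeon enemies that are activated and deactivated as Mass actors.
; Mass activation and deactivation start and stop the StateTree AI logic on the AI controller, when both are valid.
; Damage events spawn a Niagara effect at the impact point, oriented along the damage direction.
; Death handling hands off to KillEnemy with a fixed value.
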(event `self.ReceivedDamage`
  (params (Damage :type "Float (single-precision)") (ImpactPoint :type "Vector Structure (by ref)") (DamageDirection :type "Vector Structure (by ref)"))
  (`NiagaraFunctionLibrary.SpawnSystemAtLocation` "/Game/ThirdPerson/Variant_Combat/VFX/NS_Damage.NS_Damage" ImpactPoint (`KismetMathLibrary.Conv_VectorToRotator` DamageDirection)))

(event `self.OnMassActorActivated`
  (bind _returnvalue (`AIBlueprintHelperLibrary.GetAIController` self))
  (bind _returnvalue_2 (`self.GetComponentByClass` _returnvalue "/Script/GameplayStateTreeModule.StateTreeAIComponent"))
  (`/Engine/EditorBlueprintResources/StandardMacros.IsValid` _returnvalue
    (:`Is Valid`
      (`/Engine/EditorBlueprintResources/StandardMacros.IsValid` _returnvalue_2
        (:`Is Valid`
          (`BrainComponent.StartLogic` _returnvalue_2))))))

(event `self.OnMassActorDeactivated`
  (bind _returnvalue (`AIBlueprintHelperLibrary.GetAIController` self))
  (bind _returnvalue_2 (`self.GetComponentByClass` _returnvalue "/Script/GameplayStateTreeModule.StateTreeAIComponent"))
  (`/Engine/EditorBlueprintResources/StandardMacros.IsValid` _returnvalue
    (:`Is Valid`
      (`/Engine/EditorBlueprintResources/StandardMacros.IsValid` _returnvalue_2
        (:`Is Valid`
          (`BrainComponent.StopLogic` _returnvalue_2 ""))))))

(event `HandleDeath`
  (`self.KillEnemy` 5.0))

(fn `UserConstructionScript`)